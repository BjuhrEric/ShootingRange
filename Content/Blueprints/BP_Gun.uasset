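; BP_Gun is a handheld gun that motion-controller interactors can highlight, pick up and fire.
; Pickup toggles between snapping the gun to the interactor and releasing its Handle to physics; hover toggles highlight visibility while unheld.
; Firing spawns a scaled-down BP_InteractiveStaticMeshActor at Firepoint, launched by a velocity-change impulse with random pitch/yaw spread and a limited lifespan.
; Shots also play haptics on the holding hand.
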(event `self.ReceiveBeginPlay`)

(fn `GetClosestComponentData`
  (params (Interactor :type "/Game/Blueprints/BPC_WorldInteractor Object Reference"))
  (returns (Point :type "Vector Structure") (Priority :type Integer) (Component :type "SceneComponent Object Reference"))
  (return (`PrimitiveComponent.GetClosestPointOnCollision` (`self.Handle`) (`SceneComponent.K2_GetComponentLocation` Interactor) "None") 0 (`self.Handle`)))

(fn `OnDrag`
  (params (Interactor :type "/Game/Blueprints/BPC_WorldInteractor Object Reference"))
  (returns (Return :type Boolean))
  (return false))

(fn `OnDragStart`
  (params (Interactor :type "/Game/Blueprints/BPC_WorldInteractor Object Reference"))
  (returns (Return :type Boolean))
  (return false))

(fn `OnDragStop`
  (params (Interactor :type "/Game/Blueprints/BPC_WorldInteractor Object Reference"))
  (returns (Return :type Boolean))
  (return false))

(fn `OnHover`
  (params (Interactor :type "/Game/Blueprints/BPC_WorldInteractor Object Reference"))
  (returns (Return :type Boolean))
  (`/Engine/EditorBlueprintResources/StandardMacros.IsValid` (`self.Interactor`)
    (:`Is Valid`
      _)
    (:`Is Not Valid`
      (`SceneComponent.ToggleVisibility` (`self.HandleHighlighted`) false)
      (`SceneComponent.ToggleVisibility` (`self.Handle`) false)))
  (return false))

(fn `OnHoveredComponentChanged`
  (params (Interactor :type "/Game/Blueprints/BPC_WorldInteractor Object Reference") (OldComponent :type "SceneComponent Object Reference") (NewComponent :type "SceneComponent Object Reference"))
  (returns (Return :type Boolean))
  (return false))

(fn `OnPickupPressed`
  (params (Interactor :type "/Game/Blueprints/BPC_WorldInteractor Object Reference"))
  (returns (Return :type Boolean))
  (bind _interactor (`self.Interactor`))
  (bind _handle (`self.Handle`))
  (if (and (== Interactor _interactor) (`KismetSystemLibrary.IsValid` _interactor))
    ;[1 1 1] Drop
    (set `self.Interactor` null)
    (`PrimitiveComponent.SetSimulatePhysics` (`self.Handle`) true)
    (else
      ;[1 1 1] Pickup
      (set `self.Interactor` Interactor)
      (`PrimitiveComponent.SetSimulatePhysics` _handle false)
      (`SceneComponent.K2_AttachToComponent` _handle (`self.GunRoot`) "None" "SnapToTarget" "SnapToTarget" "KeepWorld" true)
      (`self.K2_AttachToComponent` (`self.Interactor`) "None" "SnapToTarget" "SnapToTarget" "KeepWorld")))
  (return false))

(fn `OnPickupReleased`
  (params (Interactor :type "/Game/Blueprints/BPC_WorldInteractor Object Reference"))
  (returns (Return :type Boolean))
  (return false))

(fn `OnUnhover`
  (params (Interactor :type "/Game/Blueprints/BPC_WorldInteractor Object Reference"))
  (returns (Return :type Boolean))
  (`/Engine/EditorBlueprintResources/StandardMacros.IsValid` (`self.Interactor`)
    (:`Is Valid`
      _)
    (:`Is Not Valid`
      (`SceneComponent.ToggleVisibility` (`self.HandleHighlighted`) false)
      (`SceneComponent.ToggleVisibility` (`self.Handle`) false)))
  (return false))

(fn `OnUsePressed`
  (params (Interactor :type "/Game/Blueprints/BPC_WorldInteractor Object Reference"))
  (returns (Return :type Boolean))
  (bind _interactor (`self.Interactor`))
  (bind _pitchspread (`self.PitchSpread`))
  (bind _yawspread (`self.YawSpread`))
  (bind (_returnvalue_location _returnvalue_rotation) (`KismetMathLibrary.BreakTransform` (`SceneComponent.K2_GetComponentToWorld` (`self.Firepoint`))))
  ;[1 1 1] Spawn bullet
  (bind _returnvalue (`|SpawnActorFromClass` "/Game/Blueprints/BP_InteractiveStaticMeshActor.BP_InteractiveStaticMeshActor_C" (`KismetMathLibrary.MakeTransform` _returnvalue_location _returnvalue_rotation (0.025 0.025 0.025)) "AlwaysSpawn" "OverrideRootScale" null null))
  (`PrimitiveComponent.AddImpulse` (`StaticMeshActor.StaticMeshComponent` _returnvalue) (* (`KismetMathLibrary.GreaterGreater_VectorRotator` (`SceneComponent.GetForwardVector` (`self.Firepoint`)) (`KismetMathLibrary.MakeRotator` 0.0 (`KismetMathLibrary.RandomFloatInRange` (* _pitchspread -1.0) _pitchspread) (`KismetMathLibrary.RandomFloatInRange` (* _yawspread -1.0) _yawspread))) (`self.BulletSpeed`)) "None" true)
  (`self.SetLifeSpan` _returnvalue 10.0)
  (`/Engine/EditorBlueprintResources/StandardMacros.IsValid` _interactor
    (:`Is Valid`
      (`PlayerController.PlayHapticEffect` (`GameplayStatics.GetPlayerController` 0) "/Game/SjolieVRTemplates/EpicContent/VirtualRealityTemplate/Blueprints/MotionControllerHaptics.MotionControllerHaptics" (`/Game/Blueprints/BPC_WorldInteractor.hand` _interactor) 1.0 false))
    (:`Is Not Valid`
      _))
  (return false))

(fn `OnUseReleased`
  (params (Interactor :type "/Game/Blueprints/BPC_WorldInteractor Object Reference"))
  (returns (Return :type Boolean))
  (return false))

(fn `UserConstructionScript`)